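; BP_ClayCharacter is a clay character Blueprint with a mouse-wheel zoom camera and switchable appearance.
; The mouse wheel steps the SpringArm arm length, clamped between a minimum and maximum distance.
; Number keys 1 to 3 swap the Mesh between normal, dark and sad Clayman skeletal meshes without resetting the pose.
; An unconnected right-mouse check for camera movement never runs.
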(event `Key|MouseScrollUp`
  (params (Key :type "Key Structure"))
  (bind _springarm (`self.SpringArm`))
  ;[1 1 1] Change Camera Zoom
  (:`Pressed`
    (set `SpringArmComponent.TargetArmLength` (`KismetMathLibrary.FMax` (- (`SpringArmComponent.TargetArmLength` _springarm) 20.0) 200.0) _springarm)))

(event `Key|MouseScrollDown`
  (params (Key :type "Key Structure"))
  (bind _springarm (`self.SpringArm`))
  ;[1 1 1] Change Camera Zoom
  (:`Pressed`
    (set `SpringArmComponent.TargetArmLength` (`KismetMathLibrary.FMin` (+ (`SpringArmComponent.TargetArmLength` _springarm) 20.0) 1000.0) _springarm)))

(event `Key|One`
  (params (Key :type "Key Structure"))
  (:`Pressed`
    (`SkinnedMeshComponent.SetSkinnedAssetAndUpdate` (`self.Mesh`) "/Game/clayman.clayman" false)))

(event `Key|Two`
  (params (Key :type "Key Structure"))
  (:`Pressed`
    (`SkinnedMeshComponent.SetSkinnedAssetAndUpdate` (`self.Mesh`) "/Game/clayman_dark.clayman_dark" false)))

(event `Key|Three`
  (params (Key :type "Key Structure"))
  (:`Pressed`
    (`SkinnedMeshComponent.SetSkinnedAssetAndUpdate` (`self.Mesh`) "/Game/clayman_sad.clayman_sad" false)))

(fn `UserConstructionScript`)